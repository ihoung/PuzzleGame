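; Interactable diary actor for Puzzle 2 that the player opens, examines and answers by entering a year.
; The first interaction plays a GeometryCache opening animation and reveals an input widget; later ones blend the view to the diary, swapping player control for cursor input until Tab exits.
; The widget's text-committed dispatcher checks the year, and a correct answer moves the camera to InvolvePosition, blends back into it and activates a page effect.
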(event `self.ReceiveBeginPlay`
  (bind _inputwidget (`self.InputWidget`))
  (`SceneComponent.SetVisibility` _inputwidget false false)
  (bind _asdairy_input_widget (cast `/Game/UI/DairyInputWidget` (`WidgetComponent.GetUserWidgetObject` _inputwidget)))
  (add `/Game/UI/DairyInputWidget.TextCommittedDispatcher` _asdairy_input_widget (delegate `CheckAnswer`)))

(event `CheckAnswer`
  (params (Year :type Integer))
  (if (== Year (`self.AnswerYear`))
    (`self.Resolve`)))

(event `self.Interact`
  (bind _geometrycache (`self.GeometryCache`))
  (if (`self.IsDairyOpened`)
    (`self.LookAtDiary`)
    (else
      (bind _asmain_scene_hud (cast `MainSceneHUD` (`PlayerController.GetHUD` (`GameplayStatics.GetPlayerController` 0))))
      (`MainSceneHUD.HideInteractionHint` _asmain_scene_hud)
      (`GeometryCacheComponent.Play` _geometrycache)
      (`KismetSystemLibrary.RetriggerableDelay` (`GeometryCacheComponent.GetDuration` _geometrycache))
      (`GeometryCacheComponent.Stop` _geometrycache)
      (set `self.IsDairyOpened` true)
      (`SceneComponent.SetVisibility` (`self.InputWidget`) true false))))

(event `self.ShowInteractionHint`
  (if (not (`GeometryCacheComponent.IsPlaying` (`self.GeometryCache`)))
    (bind _asmain_scene_hud (cast `MainSceneHUD` (`PlayerController.GetHUD` (`GameplayStatics.GetPlayerController` 0))))
    (if (`self.IsDairyOpened`)
      (`MainSceneHUD.ShowInteractionHint` _asmain_scene_hud "Interact" (`self.InteractionName_2`))
      (else
        (`MainSceneHUD.ShowInteractionHint` _asmain_scene_hud "Interact" (`self.InteractionName_1`))))))

(event `self.HideInteractionHint`
  (bind _asmain_scene_hud (cast `MainSceneHUD` (`PlayerController.GetHUD` (`GameplayStatics.GetPlayerController` 0))))
  (`MainSceneHUD.HideInteractionHint` _asmain_scene_hud))

(event `Key|Tab`
  (params (Key :type "Key Structure"))
  (:`Pressed`
    (set `self.IsExitKeyPressed` true))
  (:`Released`
    (if (`self.IsExitKeyPressed`)
      (set `self.IsExitKeyPressed` false)
      (`self.ResetView`))))

(event `Resolve`
  (`PlayerController.SetViewTargetWithBlend` (`GameplayStatics.GetPlayerController` 0) (`GameplayStatics.GetPlayerCharacter` 0) 0.3 "VTBlend_Linear" 0.0 false)
  (`KismetSystemLibrary.RetriggerableDelay` 0.3)
  (`SceneComponent.K2_SetWorldLocation` (`self.Camera`) (`SceneComponent.K2_GetComponentLocation` (`self.InvolvePosition`)) false false)
  (`KismetSystemLibrary.RetriggerableDelay` 0.2)
  (`PlayerController.SetViewTargetWithBlend` (`GameplayStatics.GetPlayerController` 0) self 3.0 "VTBlend_Linear" 0.0 false)
  (`ActorComponent.SetActive` (`self.PageEffect`) true false))

(fn `LookAtDiary`
  (bind _returnvalue (`GameplayStatics.GetPlayerController` 0))
  (`PlayerController.SetViewTargetWithBlend` _returnvalue self 1.0 "VTBlend_Linear" 0.0 false)
  (set `self.FocusState` true)
  (`|ExecutionSequence`
    (:`then_0`
      (bind _asfirst_person_character (cast `FirstPersonCharacter` (`GameplayStatics.GetPlayerCharacter` 0)))
      (`FirstPersonCharacter.SetDetectionHitActive` _asfirst_person_character false)
      (`self.DisableInput` _asfirst_person_character null))
    (:`then_1`
      (bind _asmain_scene_hud (cast `MainSceneHUD` (`PlayerController.GetHUD` _returnvalue)))
      (`MainSceneHUD.ShowInteractionHint` _asmain_scene_hud "Focus" ""))
    (:`then_2`
      (`self.EnableInput` _returnvalue))
    (:`then_3`
      (set `PlayerController.bShowMouseCursor` true _returnvalue))))

(fn `ResetView`
  (bind _returnvalue (`GameplayStatics.GetPlayerController` 0))
  (if (`self.FocusState`)
    (`PlayerController.SetViewTargetWithBlend` _returnvalue (`GameplayStatics.GetPlayerCharacter` 0) 1.0 "VTBlend_Linear" 0.0 false)
    (set `self.FocusState` false)
    (`|ExecutionSequence`
      (:`then_0`
        (bind _asfirst_person_character (cast `FirstPersonCharacter` (`GameplayStatics.GetPlayerCharacter` 0)))
        (`FirstPersonCharacter.SetDetectionHitActive` _asfirst_person_character true)
        (`self.EnableInput` _asfirst_person_character null))
      (:`then_1`
        (bind _asmain_scene_hud (cast `MainSceneHUD` (`PlayerController.GetHUD` _returnvalue)))
        (`MainSceneHUD.HideInteractionHint` _asmain_scene_hud))
      (:`then_2`
        (`self.DisableInput` _returnvalue))
      (:`then_3`
        (set `PlayerController.bShowMouseCursor` false _returnvalue)))))

(fn `UserConstructionScript`)