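; Interactable gramophone actor that starts playing music when the level begins and toggles it on and off through Interact.
; PlayMusic runs the geometry cache animation and spawns the sound at the actor's location, keeping the audio component so StopMusic can halt both.
; An IsPlaying flag drives the toggle and selects the play or stop hint shown through MainSceneHUD.
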(event `self.ReceiveBeginPlay`
  (`self.PlayMusic`))

(event `self.Interact`
  (if (`self.IsPlaying`)
    (`self.StopMusic`)
    (else
      (`self.PlayMusic`))))

(event `self.ShowInteractionHint`
  (bind _asmain_scene_hud (cast `MainSceneHUD` (`PlayerController.GetHUD` (`GameplayStatics.GetPlayerController` 0))))
  (if (`self.IsPlaying`)
    (`MainSceneHUD.ShowInteractionHint` _asmain_scene_hud "Interact" (`self.InteractionStop`))
    (else
      (`MainSceneHUD.ShowInteractionHint` _asmain_scene_hud "Interact" (`self.InteractionPlay`)))))

(event `self.HideInteractionHint`
  (bind _asmain_scene_hud (cast `MainSceneHUD` (`PlayerController.GetHUD` (`GameplayStatics.GetPlayerController` 0))))
  (`MainSceneHUD.HideInteractionHint` _asmain_scene_hud))

(fn `PlayMusic`
  (`GeometryCacheComponent.Play` (`self.GeometryCache`))
  (set `self.IsPlaying` true)
  (bind _returnvalue (`GameplayStatics.SpawnSoundAtLocation` "/Game/Audios/gramophone/Gramophone.Gramophone" (`self.K2_GetActorLocation` self) (struct) 1.0 1.0 0.0 null null))
  (set `self.Music` _returnvalue))

(fn `StopMusic`
  (`GeometryCacheComponent.Stop` (`self.GeometryCache`))
  (set `self.IsPlaying` false)
  (`AudioComponent.Stop` (`self.Music`)))

(fn `UserConstructionScript`)