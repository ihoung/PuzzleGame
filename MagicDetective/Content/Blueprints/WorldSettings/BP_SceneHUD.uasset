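; BP_SceneHUD is a scene HUD actor that plays a viewport fade-in when play begins.
; On BeginPlay it creates a BP_FadeViewportWidget, shows its mask, adds it to the viewport and starts the fade.
; The widget's Z-order comes from a WidgetZOrder map keyed by widget class.
; A bound fade-finished event then hides the widget without removing it from the viewport.
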(event `FadeInFinished`
  (`Widget.SetVisibility` (`self.FadeWidget`) "Hidden"))

(event `self.ReceiveBeginPlay`
  (bind _returnvalue (`|CreateWidget` "/Game/UI/BP_FadeViewportWidget.BP_FadeViewportWidget_C"))
  (bind _output_get (set `self.FadeWidget` _returnvalue))
  (`|ExecutionSequence`
    (:`then_0`
      (add `/Game/UI/BP_FadeViewportWidget.OnFadeInFinished` _output_get (delegate `FadeInFinished`))
      (`/Game/UI/BP_FadeViewportWidget.SetMaskVisibility` _output_get true))
    (:`then_1`
      (`UserWidget.AddToViewport` _output_get (`BlueprintMapLibrary.Map_Find` (`self.WidgetZOrder`) "/Game/UI/BP_FadeViewportWidget.BP_FadeViewportWidget_C")))
    (:`then_2`
      (`/Game/UI/BP_FadeViewportWidget.FadeInViewport` _output_get))))

(fn `UserConstructionScript`)