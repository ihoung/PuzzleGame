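; Main menu HUD that plays a viewport fade-out before the game opens a new level.
; On BeginPlay it creates a hidden-mask fade widget above the viewport and listens to the existing main menu widget's start-game dispatcher.
; That dispatcher triggers the fade-out, whose finished event calls OpenNewLevel on the menu widget, so the level change waits for the fade.
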(event `ShowFadeOut`
  (bind _fadewidget (`self.FadeWidget`))
  (`/Game/UI/BP_FadeViewportWidget.SetMaskVisibility` _fadewidget true)
  (`/Game/UI/BP_FadeViewportWidget.FadeOutViewport` _fadewidget))

(event `StartGame`
  (bind _asmain_menu_widget (cast `MainMenuWidget` (`self.MainMenu`)))
  (`MainMenuWidget.OpenNewLevel` _asmain_menu_widget))

(event `self.ReceiveBeginPlay`
  (`|ExecutionSequence`
    (:`then_0`
      (bind _asbp_main_menu_widget (cast `/Game/UI/BP_MainMenuWidget` (`self.MainMenu`)))
      (add `/Game/UI/BP_MainMenuWidget.StartGameEventDispatcher` _asbp_main_menu_widget (delegate `ShowFadeOut`)))
    (:`then_1`
      (bind _returnvalue (`|CreateWidget` "/Game/UI/BP_FadeViewportWidget.BP_FadeViewportWidget_C"))
      (bind _output_get (set `self.FadeWidget` _returnvalue))
      (`|ExecutionSequence`
        (:`then_0`
          (add `/Game/UI/BP_FadeViewportWidget.OnFadeOutFinished` _output_get (delegate `StartGame`))
          (`/Game/UI/BP_FadeViewportWidget.SetMaskVisibility` _output_get false))
        (:`then_1`
          (`UserWidget.AddToViewport` _output_get 10))))))

(fn `UserConstructionScript`)